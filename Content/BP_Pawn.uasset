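; Pawn that joins a team on BeginPlay and tints its mesh to show which team it is in.
; A TeamNumber switch sets TempTeam, which is assigned after an optional random delay, either through its CustomAIController or directly on the pawn.
; The construction script creates a dynamic material instance, which RefreshColor recolors by team name (Purple, Orange or Yellow).
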(event `self.ReceiveBeginPlay`
  (switch `int` (`self.TeamNumber`)
    (:`0`
      (set `self.TempTeam` (struct :`Name` "Purple")))
    (:`1`
      (set `self.TempTeam` (struct :`Name` "Orange")))
    (:`2`
      (set `self.TempTeam` (struct :`Name` "Yellow"))))
  ;[1 1 1] Randomizing delay of setting up teams.
  (if (`self.RandomizeDelayOfSettingTeams`)
    (set `self.Delay` (`KismetMathLibrary.RandomFloatInRange` 1.0 3.0))
    (else
      (set `self.Delay` 0.0)))
  (`KismetSystemLibrary.Delay` (`self.Delay`))
  ;[1 1 1] Assigning pawn/controller to Team
  (if (`self.SetTeamViaController`)
    (cast `CustomAIController` (`self.GetController`))
    (`self.SetTeam` (`self.TempTeam`))
    (else
      (`self.SetTeam` (`self.TempTeam`))))
  ;[1 1 1] Just to see what Pawn is in what Team
  (`self.RefreshColor`))

(fn `RefreshColor`
  (bind _dmi (`self.DMI`))
  (bind _paramname (`self.ParamName`))
  (bind (_outname _returnvalue) (`CustomTypes.GetTeamName` self))
  (if _returnvalue
    (switch `name` _outname
      (:`Purple`
        (`MaterialInstanceDynamic.SetVectorParameterValue` _dmi _paramname (struct :`R` 0.475 :`B` 0.437275 :`A` 1.0)))
      (:`Orange`
        (`MaterialInstanceDynamic.SetVectorParameterValue` _dmi _paramname (struct :`R` 1.0 :`G` 0.368699 :`A` 1.0)))
      (:`Yellow`
        (`MaterialInstanceDynamic.SetVectorParameterValue` _dmi _paramname (struct :`R` 0.929934 :`G` 1.0 :`A` 1.0))))))

(fn `UserConstructionScript`
  (`/Engine/EditorBlueprintResources/StandardMacros.IsValid` (`self.DMI`)
    (:`Is Valid`
      _)
    (:`Is Not Valid`
      (bind _returnvalue (`PrimitiveComponent.CreateDynamicMaterialInstance` (`self.Mesh`) 0 "/Game/Misc/M_PawnBase.M_PawnBase"))
      (bind _output_get (set `self.DMI` _returnvalue))))
  (`PrimitiveComponent.SetMaterial` (`self.Mesh`) 0 _output_get))